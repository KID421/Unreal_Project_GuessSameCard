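; BP_GameManager is a manager Blueprint that deals a grid of cards when its Cube component is clicked.
; Nested loops spawn four BP_Card actors in a 2x2 layout on the Y-Z plane and add each to a card array (卡片物件陣列).
; Each iteration also sets a material-not-yet-chosen flag (還沒選擇材質), which is never read here, and the material array (材質球陣列) is unused.
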(event `self.Cube.OnClicked`
  (params (TouchedComponent :type "PrimitiveComponent Object Reference") (ButtonPressed :type "Key Structure"))
  (for _index (range 2)
    (for _index_2 (range 2)
      (set `self.還沒選擇材質` true)
      (bind _returnvalue (`|SpawnActorFromClass` "/Game/BP/BP_Card.BP_Card_C" (`KismetMathLibrary.MakeTransform` (`KismetMathLibrary.MakeVector` 600.0 (`KismetMathLibrary.Conv_IntToDouble` (* (mod _index 2) 150)) (`KismetMathLibrary.Conv_IntToDouble` (* (mod _index_2 2) -150)))) "Undefined" "OverrideRootScale" null null null))
      (`KismetArrayLibrary.Array_Add` (`self.卡片物件陣列`) _returnvalue))))

(fn `UserConstructionScript`)